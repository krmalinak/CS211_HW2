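; BP_Celestial_Body is a celestial body actor that orbits the actor it is attached to.
; The construction script applies its BodyMaterial and sets a uniform actor scale from Scale.
; Each tick, if an attach parent exists, it rotates its offset from that parent's owner in yaw by RevolutionRate and moves there without sweeping.
; The revolution step is not scaled by delta time, so orbit speed depends on frame rate.
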(event EventTick
  (params (DeltaSeconds :type Float%20%28single-precision%29))
  (bind _returnvalue (Transformation|GetAttachParent))
  ;[1 1 1] validate parent
  (Utilities|IsValid _returnvalue
    (:Is%20Valid
      (Variables|Default|SetParent (Components|GetOwner _returnvalue))
      (Transformation|SetActorLocation (+ (Math|Vector|RotateVector (- (Transformation|GetActorLocation) (Transformation|GetActorLocation (Variables|Default|GetParent))) (Class|KismetMathLibrary|MakeRot 0.0 (Variables|Default|GetRevolutionRate) 0.0)) (Transformation|GetActorLocation (Variables|Default|GetParent))) false))))

(fn ConstructionScript
  (Rendering|Material|SetMaterial 0 (Variables|Default|GetBodyMaterial))
  (Transformation|SetActorScale3D (Math|Conversions|ToVector(Float) (Variables|Default|GetScale))))
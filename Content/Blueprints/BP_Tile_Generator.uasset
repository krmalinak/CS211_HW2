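; Tile generator actor that fills an X by Y by Z grid with copies of one static mesh.
; The construction script adds a static mesh component per cell under RootCube, placed by Space and sized by a uniform Scale.
; Each copy gets a random upward height offset and random rotation within the variation limits, rerolled whenever construction runs.
; An older 2D X-Y version remains unconnected, and the event graph is empty.
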(event EventBeginPlay)

(event EventActorBeginOverlap
  (params (OtherActor :type Actor%20Object%20Reference)))

(event EventTick
  (params (DeltaSeconds :type Float%20%28single-precision%29)))

(fn ConstructionScript
  (bind _rotationvariation (Variables|Default|GetRotationVariation))
  (bind _space (Variables|Default|GetSpace))
  ;[1 1 1] validate XY bounds
  (if (Math|Boolean|ANDBoolean (> (Variables|Default|GetX) 0) (> (Variables|Default|GetY) 0) (> (Variables|Default|GetZ) 0))
    (for _index (range 0 (- (Variables|Default|GetX) 1))
      (for _index_2 (range 0 (- (Variables|Default|GetY) 1))
        (for _index_3 (range 0 (- (Variables|Default|GetZ) 1))
          (bind _returnvalue (AddComponent|AddStaticMeshComponent true))
          (Components|StaticMesh|SetStaticMesh _returnvalue (Variables|Default|GetMyStaticMesh))
          (Class|SceneComponent|Attachto _returnvalue (Variables|Default|Getroot_cube) "None" "KeepRelativeOffset" true)
          (Transformation|SetRelativeTransform _returnvalue (Math|Transform|MakeTransform (Math|Vector|MakeVector (* _index _space) (* _index_2 _space) (+ (* _index_3 _space) (Math|Random|RandomFloatinRange 0.0 (Variables|Default|GetHeightVariation)))) (Class|KismetMathLibrary|MakeRot (Math|Random|RandomFloatinRange 0.0 _rotationvariation) (Math|Random|RandomFloatinRange 0.0 _rotationvariation) (Math|Random|RandomFloatinRange 0.0 _rotationvariation)) (Math|Conversions|ToVector(Float) (Variables|Default|GetScale))) false))))))
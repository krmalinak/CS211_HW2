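; BP_Spline_Tool is a construction-script tool that scatters randomly chosen static meshes at regular intervals along a spline.
; It steps along the spline by MeshInterval, adding a mesh component at each point, aligned to the spline's rotation with a uniform Scale.
; A helper picks random indices into the mesh and material arrays for each instance, setting material slot 0.
; Randomness is unseeded, so construction reruns reshuffle the results.
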(fn ConstructionScript
  (bind _meshinterval (Variables|Default|GetMeshInterval))
  (bind _mystaticmeshes (Variables|Default|GetMyStaticMeshes))
  (bind _spline (Variables|Default|GetSpline))
  (bind _mymaterials (Variables|Default|GetMyMaterials))
  (for _index (range 0 (Math|Float|Floor (/ (Spline|GetSplineLength (Variables|Default|GetSpline)) _meshinterval)))
    (bind _returnvalue (AddComponent|AddStaticMeshComponent true))
    (bind _index_2 (CallFunction|GetRandIndexinRange (Utilities|Array|Length _mystaticmeshes)))
    (Components|StaticMesh|SetStaticMesh _returnvalue (Utilities|Array|Get(acopy) _mystaticmeshes _index_2))
    (Class|SceneComponent|Attachto _returnvalue (Variables|Default|GetRoot) "None" "KeepRelativeOffset" true)
    (Transformation|SetWorldTransform _returnvalue (Math|Transform|MakeTransform (Class|SplineComponent|GetWorldLocationatDistanceAlongSpline _spline (* _index _meshinterval)) (Class|SplineComponent|GetWorldRotationatDistanceAlongSpline _spline (* _index _meshinterval)) (Math|Conversions|ToVector(Float) (Variables|Default|GetScale))) false)
    (bind _index_3 (CallFunction|GetRandIndexinRange (Utilities|Array|Length _mymaterials)))
    (Rendering|Material|SetMaterial _returnvalue 0 (Utilities|Array|Get(acopy) _mymaterials _index_3))))

(fn GetRandIndexinRange
  (params (Length :type Integer))
  (return (Math|Random|RandomIntegerinRange 0 (- Length 1))))